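; Maze actor that generates a random maze at BeginPlay and reveals it tile by tile, then shows the HUD's Spawn AI button.
; GenerateMaze uses seeded recursive backtracking, carving two-cell steps joined by bridge tiles and recording dead ends.
; BlockByBlockSpawning spawns path, end-path and wall actors under container actors, storing dead-end locations.
; GenerateFinishLineWalls adds four scaled border finish lines; BlockByBlock then unhides stored tiles on a short delay loop.
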(event `self.ReceiveBeginPlay`
  (bind (_size_x _size_y) (break `IntPoint` (`self.Size`)))
  ;[1 1 1] Storing Refernce
  (bind _asbp_third_person_game_mode (cast `/Game/ThirdPerson/Blueprints/BP_ThirdPersonGameMode` (`GameplayStatics.GetGameMode`)))
  (set `self.MyGameMode` _asbp_third_person_game_mode)
  (bind _asmaze_task_hudclass (cast `/Game/MazeTask/UI/MazeTaskHUDClass` (`PlayerController.GetHUD` (`GameplayStatics.GetPlayerController` 0))))
  (set `self.HUDRef` _asmaze_task_hudclass)
  ;[1 1 1 1 14] Remove Old Instances
  (message `/Game/MazeTask/MT_Blueprints/BPI_IntanceManager.RemoveAll_Instances` (`self.InsatanceManager`))
  (set `self.Size` (make `IntPoint` (* (/ _size_x 2) 2) (* (/ _size_y 2) 2)))
  (bind (_pathtilesout _endpathsout) (`self.GenerateMaze` (`self.Size`) (`KismetMathLibrary.RandomIntegerInRange` 0 19)))
  (set `self.Path Tiles` _pathtilesout)
  (set `self.End Paths` _endpathsout)
  (`self.Block_By_Block_Spawning`)
  (`self.GenerateFinishLineWalls`)
  (`self.BlockByBlock`))

(event `BlockByBlock`
  (bind _spawnai_btn (`/Game/MazeTask/UI/MainWidget.SpawnAI_Btn` (`/Game/MazeTask/UI/MazeTaskHUDClass.MainWidgetRef` (`self.HUDRef`))))
  ;[1 1 1] Show the Maze creation block by block
  (set `self.LastSpawnObject` (`KismetArrayLibrary.Array_LastIndex` (`self.PathTilesArray`)))
  (if (`self.AllSpawn`) :!label _label
    _
    (elif (== (`self.AllSpawnIndex`) (`self.LastSpawnObject`))
      (`self.SetActorHiddenInGame` (`|GetArrayItem` (`self.PathTilesArray`) (`self.AllSpawnIndex`)) false)
      (set `self.AllSpawn` true)
      (`/Engine/EditorBlueprintResources/StandardMacros.IsValid` _spawnai_btn
        (:`Is Valid`
          (`Widget.SetVisibility` _spawnai_btn "Visible")))
      (else
        (`KismetSystemLibrary.Delay` 0.01)
        (`self.SetActorHiddenInGame` (`|GetArrayItem` (`self.PathTilesArray`) (`self.AllSpawnIndex`)) false)
        (set `self.AllSpawnIndex` (+ (`self.AllSpawnIndex`) 1))
        (goto _label)))))

(fn `AddNeighbourLoc`
  (params (Size :type "IntPoint Structure (by ref)") (RandStream :type "RandomStream Structure (by ref)") (CurrentLoc :type "IntPoint Structure (by ref)") (PathTiles :type "Set of IntPoint Structure (by ref)") (BridgeTiles :type "Set of IntPoint Structure (by ref)") (ToCheck :type "Set of IntPoint Structure (by ref)") (EndPaths :type "Set of IntPoint Structure (by ref)"))
  (locals (NeighbourIndex :type Integer))
  (bind (_floor _bridge) (`self.GetNeighbourAndBridge` (`local.CurrentLoc`) (`local.NeighbourIndex`)))
  (bind _returnvalue (+ (`local.NeighbourIndex`) 1))
  (set `local.NeighbourIndex` (`KismetMathLibrary.RandomIntegerInRangeFromStream` 0 3 (`local.RandStream`)))
  (if (`self.CheckIsValidLocation` (`self.GetNeighbourAndBridge` (`local.CurrentLoc`) (`local.NeighbourIndex`)) (`local.Size`) (`local.PathTiles`) (`local.BridgeTiles`)) :!label _label
    (`BlueprintSetLibrary.Set_Add` (`local.PathTiles`) _floor)
    (`BlueprintSetLibrary.Set_Add` (`local.BridgeTiles`) _bridge)
    (`BlueprintSetLibrary.Set_Add` (`local.ToCheck`) _floor)
    (`self.AddNeighbourLoc` (`local.Size`) (`local.RandStream`) _floor (`local.PathTiles`) (`local.BridgeTiles`) (`local.ToCheck`) (`local.EndPaths`))
    (else
      (`/Game/MazeTask/MT_Blueprints/CustomMacroLibrary.Do N+` 4
        (:`Exit`
          (set `local.NeighbourIndex` (`KismetMathLibrary.SelectInt` 0 _returnvalue (>= _returnvalue 4)))
          (goto _label))
        (:`Over Nth`
          (bind _count (`self.GetNeighbourCount` (`local.CurrentLoc`) (`local.PathTiles`)))
          (if (== _count 1)
            (`BlueprintSetLibrary.Set_Add` (`local.EndPaths`) (`local.CurrentLoc`))))))))

(fn `BackTrace`
  (params (CurrentTile :type "IntPoint Structure (by ref)") (ToCheck :type "Set of IntPoint Structure (by ref)") (BridgeTiles :type "Set of IntPoint Structure (by ref)") (PathTiles :type "Set of IntPoint Structure (by ref)"))
  (bind _result (`BlueprintSetLibrary.Set_ToArray` ToCheck))
  (bind _output (`|GetArrayItem` _result (`KismetArrayLibrary.Array_LastIndex` _result)))
  (`|VariableSetRef` (`local.CurrentTile`) _output)
  (`BlueprintSetLibrary.Set_Remove` (`local.ToCheck`) _output)
  (bind _result_2 (`BlueprintSetLibrary.Set_ToArray` (`local.BridgeTiles`)))
  (bind _output_2 (`|GetArrayItem` _result_2 (`KismetArrayLibrary.Array_LastIndex` _result_2)))
  (`BlueprintSetLibrary.Set_Add` (`local.PathTiles`) _output_2)
  (`BlueprintSetLibrary.Set_Remove` (`local.BridgeTiles`) _output_2))

(fn `Block_By_Block_Spawning`
  (locals (`Loop Index` :type Integer) (SegmentIndex :type "Array of Boolean") (EndPoints_Index :type Integer) (WallPointsIndex :type Integer) (AddArrayIndex :type Integer))
  (bind (_size_x _size_y) (break `IntPoint` (`self.Size`)))
  (for _index (range (+ _size_x 1))
    (for _index_2 (range (+ _size_y 1))
      (set `self.LoopLoc` (make `IntPoint` _index _index_2))
      ;[1 1 1] Checks If Maze has space to spawn
      (if (`BlueprintSetLibrary.Set_Contains` (`self.Path Tiles`) (`self.LoopLoc`))
        ;[0.2031 0.08359 0.08146] PATHWAY - FloorTiles Generation
        ;;[1 1 1] Checks if Location has End Path
        (if (`BlueprintSetLibrary.Set_Contains` (`self.End Paths`) (`self.LoopLoc`))
          ;;[1 1 1] Current Spawning Location Has end Path, can spawn other tile here for representation
          (bind _returnvalue (`|SpawnActorFromClass` "/Game/MazeTask/MT_Blueprints/MT_PathEndTile.MT_PathEndTile_C" (`self.BuildTileLocation` (`self.LoopLoc`)) "Undefined" "OverrideRootScale" null (`self.Instigator`)))
          ;;[1 1 1] Keep Record of Spawning Objects
          (`KismetArrayLibrary.Array_Set` (`self.PathTilesArray`) (`local.AddArrayIndex`) _returnvalue true)
          (set `local.AddArrayIndex` (+ 1 (`local.AddArrayIndex`)))
          ;;[1 1 1] For Ease, Set Walls Actor as a Child to a Parent Actor
          (`self.K2_AttachToActor` _returnvalue (`self.EndPathContainer`) "None" "KeepWorld" "KeepWorld" "KeepWorld" true)
          ;;[1 1 1] Create Map and Store End paths for getting their locations
          (bind _output_get (set `local.EndPoints_Index` (+ 1 (`local.EndPoints_Index`))))
          (`BlueprintMapLibrary.Map_Add` (`self.EndPointsLocation`) _output_get (`self.K2_GetActorLocation` _returnvalue))
          (else
            ;;[1 1 1] Current Spawning Location Has way for Path, can spawn Different tiles here for representation
            (bind _returnvalue_2 (`|SpawnActorFromClass` "/Game/MazeTask/MT_Blueprints/MT_PathTile.MT_PathTile_C" (`self.BuildTileLocation` (`self.LoopLoc`)) "Undefined" "OverrideRootScale" null (`self.Instigator`)))
            ;;[1 1 1] Keep Record of Spawning Objects
            (`KismetArrayLibrary.Array_Set` (`self.PathTilesArray`) (`local.AddArrayIndex`) _returnvalue_2 true)
            (set `local.AddArrayIndex` (+ 1 (`local.AddArrayIndex`)))
            ;;[1 1 1] For Ease, Set Walls Actor as a Child to a Parent Actor
            (`self.K2_AttachToActor` _returnvalue_2 (`self.PathContainer`) "None" "KeepWorld" "KeepWorld" "KeepWorld" true)))
        (else
          ;[0.1667 0.1113 0.01103] Walls Generation
          ;;[1 1 1] Spawn Walls
          (bind _returnvalue_3 (`|SpawnActorFromClass` "/Game/MazeTask/MT_Blueprints/MT_Wall.MT_Wall_C" (`self.BuildTileLocation` (`self.LoopLoc`)) "Undefined" "OverrideRootScale" null (`self.Instigator`)))
          ;;[1 1 1] Keep Record of Spawning Objects
          (`KismetArrayLibrary.Array_Set` (`self.PathTilesArray`) (`local.AddArrayIndex`) _returnvalue_3 true)
          ;;[1 1 1] For Ease, Set Walls Actor as a Child to a Parent Actor
          (set `local.AddArrayIndex` (+ 1 (`local.AddArrayIndex`)))
          (`self.K2_AttachToActor` _returnvalue_3 (`self.WallsContainer`) "None" "KeepWorld" "KeepWorld" "KeepWorld" true))))))

(fn `FindMiddlePoint`
  (returns (`Mid X` :type "Float (double-precision)") (`Mid Y` :type "Float (double-precision)"))
  (bind (_size_x _size_y) (break `IntPoint` (`self.Size`)))
  ;[1 1 1] Return Middle Point of the Maze
  (return (+ (* (/ (+ _size_x 1) 2) (`self.TileSize`)) 5.0) (+ (* (/ (+ _size_y 1) 2) (`self.TileSize`)) 5.0)))

(fn `GenerateFinishLineWalls`
  (locals (Index :type Integer) (Lenght_x :type Integer) (Width_y :type Integer) (Horizontal_Pos_x :type "Float (double-precision)") (Verical_Pos_y :type "Float (double-precision)"))
  (bind (_size_x _size_y) (break `IntPoint` (`self.Size`)))
  (bind _returnvalue (`KismetMathLibrary.MakeVector` (`KismetMathLibrary.Conv_IntToDouble` (`local.Width_y`)) 1.0 2.0))
  (set `local.Lenght_x` (+ _size_x 1))
  (set `local.Width_y` (+ _size_y 1))
  (set `local.Horizontal_Pos_x` (* (`local.Lenght_x`) (`self.TileSize`)))
  (set `local.Verical_Pos_y` (* (`local.Width_y`) (`self.TileSize`)))
  (for _index (range 4)
    (set `local.Index` _index)
    (`|SpawnActorFromClass` "/Game/MazeTask/MT_Blueprints/BP_FinishLine.BP_FinishLine_C" (`KismetMathLibrary.MakeTransform` (select `int` (`local.Index`) :`0` (0.0 0.0 0.0) :`1` (0.0 0.0 0.0) :`2` (`KismetMathLibrary.MakeVector` (`local.Horizontal_Pos_x`) (`local.Verical_Pos_y`)) :`3` (`KismetMathLibrary.MakeVector` (`local.Horizontal_Pos_x`) (`local.Verical_Pos_y`))) (select `int` (`local.Index`) :`0` (struct) :`1` (struct :`Yaw` 90.0) :`2` (struct :`Yaw` -90.0) :`3` (struct :`Yaw` 180.0) :!type "Rotator Structure") (select `int` (`local.Index`) :`0` (`KismetMathLibrary.MakeVector` (`KismetMathLibrary.Conv_IntToDouble` (`local.Lenght_x`)) 1.0 2.0) :`1` _returnvalue :`2` _returnvalue :`3` (`KismetMathLibrary.MakeVector` (`KismetMathLibrary.Conv_IntToDouble` (`local.Lenght_x`)) 1.0 2.0))) "Undefined" "OverrideRootScale" null null)))

(fn `GenerateMaze`
  (params (Size :type "IntPoint Structure") (Seed :type Integer))
  (returns (PathTilesOut :type "Set of IntPoint Structure") (EndPathsOut :type "Set of IntPoint Structure"))
  (locals (RandStream :type "RandomStream Structure") (LocalSize :type "IntPoint Structure") (StartingLoc :type "IntPoint Structure") (CurrentLoc :type "IntPoint Structure") (PathTiles :type "Set of IntPoint Structure") (BridgeTiles :type "Set of IntPoint Structure") (ToCheck :type "Set of IntPoint Structure") (EndPaths :type "Set of IntPoint Structure"))
  (`KismetMathLibrary.SetRandomStreamSeed` (`local.RandStream`) Seed)
  (set `local.LocalSize` Size)
  (set `local.StartingLoc` (`self.GetRandomLocationInBounds` (`local.LocalSize`) (`local.RandStream`)))
  (set `local.CurrentLoc` (struct))
  (`self.AddNeighbourLoc` (`local.LocalSize`) (`local.RandStream`) (`local.CurrentLoc`) (`local.PathTiles`) (`local.BridgeTiles`) (`local.ToCheck`) (`local.EndPaths`) :!label _label)
  (if (> (`BlueprintSetLibrary.Set_Length` (`local.ToCheck`)) 0)
    (`self.BackTrace` (`local.CurrentLoc`) (`local.ToCheck`) (`local.BridgeTiles`) (`local.PathTiles`))
    (goto _label)
    (else
      (return (`local.PathTiles`) (`local.EndPaths`)))))

(fn `GetNeighbourCount`
  (params (CurrentLocation :type "IntPoint Structure (by ref)") (PathTiles :type "Set of IntPoint Structure (by ref)"))
  (returns (Count :type Integer))
  (locals (Counter :type Integer))
  (for _array_element (`self.GetNeighbourLocation` CurrentLocation 1)
    (if (`BlueprintSetLibrary.Set_Contains` (`local.PathTiles`) _array_element)
      (set `local.Counter` (+ (`local.Counter`) 1))))
  (return (`local.Counter`)))

(fn `SpawnMazeMeshes`
  (locals (LoopLocation :type "IntPoint Structure") (`Loop Index` :type Integer) (SegmentIndex :type "Array of Boolean"))
  (bind (_size_x _size_y) (break `IntPoint` (`self.Size`)))
  (for _index (range (+ _size_x 1))
    (for _index_2 (range (+ _size_y 1))
      (set `local.LoopLocation` (make `IntPoint` _index _index_2))
      (if (`BlueprintSetLibrary.Set_Contains` (`self.Path Tiles`) (`local.LoopLocation`))
        ;[1 1 1] FloorTiles Generation - If has end path then spawn green tile other wise normal tile
        (message `/Game/MazeTask/MT_Blueprints/BPI_IntanceManager.AddNewMeshInstance` (`self.InsatanceManager`) (select `bool` (`BlueprintSetLibrary.Set_Contains` (`self.End Paths`) (`local.LoopLocation`)) :`false` "/Game/MazeTask/MT_Meshes/MT_Simple_GroundTile.MT_Simple_GroundTile" :`true` "/Game/MazeTask/MT_Meshes/MT_Green_GroundTile.MT_Green_GroundTile" :!type "StaticMesh Object Reference") (`self.BuildTileLocation` (`local.LoopLocation`)))
        (else
          ;[1 1 1] Walls
          (message `/Game/MazeTask/MT_Blueprints/BPI_IntanceManager.AddNewMeshInstance` (`self.InsatanceManager`) "/Game/MazeTask/MT_Meshes/Walls.Walls" (`self.BuildTileLocation` (`local.LoopLocation`) 800.0)))))))

(fn `UserConstructionScript`)