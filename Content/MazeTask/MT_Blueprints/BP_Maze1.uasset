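; Maze generator actor that builds a random grid maze of instanced floor and wall meshes at BeginPlay, using an even-snapped size and random seed.
; GenerateMaze carves paths by seeded depth-first search: AddNeighbourLoc recursively steps two cells, and BackTrace pops pending cells and bridge tiles into the path.
; Dead ends are recorded, though their floor mesh matches normal tiles.
; SpawnMazeMeshes sends floors for path cells and walls elsewhere to the instance manager.
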(event `self.ReceiveBeginPlay`
  (bind (_size_x _size_y) (break `IntPoint` (`self.Size`)))
  ;[1 1 1 1 14] Remove Old Instances
  (message `/Game/MazeTask/MT_Blueprints/BPI_IntanceManager.RemoveAll_Instances` (`self.InsatanceManager`))
  (set `self.Size` (make `IntPoint` (* (/ _size_x 2) 2) (* (/ _size_y 2) 2)))
  (bind (_pathtilesout _endpathsout) (`self.GenerateMaze` (`self.Size`) (`KismetMathLibrary.RandomIntegerInRange` 0 50)))
  (set `self.Path Tiles` _pathtilesout)
  (set `self.End Paths` _endpathsout)
  (`self.SpawnMazeMeshes`))

(fn `AddNeighbourLoc`
  (params (Size :type "IntPoint Structure (by ref)") (RandStream :type "RandomStream Structure (by ref)") (CurrentLoc :type "IntPoint Structure (by ref)") (PathTiles :type "Set of IntPoint Structure (by ref)") (BridgeTiles :type "Set of IntPoint Structure (by ref)") (ToCheck :type "Set of IntPoint Structure (by ref)") (EndPaths :type "Set of IntPoint Structure (by ref)"))
  (locals (NeighbourIndex :type Integer))
  (bind (_floor _bridge) (`self.GetNeighbourAndBridge` (`local.CurrentLoc`) (`local.NeighbourIndex`)))
  (bind _returnvalue (+ (`local.NeighbourIndex`) 1))
  (set `local.NeighbourIndex` (`KismetMathLibrary.RandomIntegerInRangeFromStream` 0 3 (`local.RandStream`)))
  (if (`self.CheckIsValidLocation` (`self.GetNeighbourAndBridge` (`local.CurrentLoc`) (`local.NeighbourIndex`)) (`local.Size`) (`local.PathTiles`) (`local.BridgeTiles`)) :!label _label
    (`BlueprintSetLibrary.Set_Add` (`local.PathTiles`) _floor)
    (`BlueprintSetLibrary.Set_Add` (`local.BridgeTiles`) _bridge)
    (`BlueprintSetLibrary.Set_Add` (`local.ToCheck`) _floor)
    (`self.AddNeighbourLoc` (`local.Size`) (`local.RandStream`) _floor (`local.PathTiles`) (`local.BridgeTiles`) (`local.ToCheck`) (`local.EndPaths`))
    (else
      (`/Game/MazeTask/MT_Blueprints/CustomMacroLibrary.Do N+` 4
        (:`Exit`
          (set `local.NeighbourIndex` (`KismetMathLibrary.SelectInt` 0 _returnvalue (>= _returnvalue 4)))
          (goto _label))
        (:`Over Nth`
          (bind _count (`self.GetNeighbourCount` (`local.CurrentLoc`) (`local.PathTiles`)))
          (if (== _count 1)
            (`BlueprintSetLibrary.Set_Add` (`local.EndPaths`) (`local.CurrentLoc`))))))))

(fn `BackTrace`
  (params (CurrentTile :type "IntPoint Structure (by ref)") (ToCheck :type "Set of IntPoint Structure (by ref)") (BridgeTiles :type "Set of IntPoint Structure (by ref)") (PathTiles :type "Set of IntPoint Structure (by ref)"))
  (bind _result (`BlueprintSetLibrary.Set_ToArray` ToCheck))
  (bind _output (`|GetArrayItem` _result (`KismetArrayLibrary.Array_LastIndex` _result)))
  (`|VariableSetRef` (`local.CurrentTile`) _output)
  (`BlueprintSetLibrary.Set_Remove` (`local.ToCheck`) _output)
  (bind _result_2 (`BlueprintSetLibrary.Set_ToArray` (`local.BridgeTiles`)))
  (bind _output_2 (`|GetArrayItem` _result_2 (`KismetArrayLibrary.Array_LastIndex` _result_2)))
  (`BlueprintSetLibrary.Set_Add` (`local.PathTiles`) _output_2)
  (`BlueprintSetLibrary.Set_Remove` (`local.BridgeTiles`) _output_2))

(fn `GenerateMaze`
  (params (Size :type "IntPoint Structure") (Seed :type Integer))
  (returns (PathTilesOut :type "Set of IntPoint Structure") (EndPathsOut :type "Set of IntPoint Structure"))
  (locals (RandStream :type "RandomStream Structure") (LocalSize :type "IntPoint Structure") (StartingLoc :type "IntPoint Structure") (CurrentLoc :type "IntPoint Structure") (PathTiles :type "Set of IntPoint Structure") (BridgeTiles :type "Set of IntPoint Structure") (ToCheck :type "Set of IntPoint Structure") (EndPaths :type "Set of IntPoint Structure"))
  (`KismetMathLibrary.SetRandomStreamSeed` (`local.RandStream`) Seed)
  (set `local.LocalSize` Size)
  (set `local.StartingLoc` (`self.GetRandomLocationInBounds` (`local.LocalSize`) (`local.RandStream`)))
  (set `local.CurrentLoc` (struct))
  (`self.AddNeighbourLoc` (`local.LocalSize`) (`local.RandStream`) (`local.CurrentLoc`) (`local.PathTiles`) (`local.BridgeTiles`) (`local.ToCheck`) (`local.EndPaths`) :!label _label)
  (if (> (`BlueprintSetLibrary.Set_Length` (`local.ToCheck`)) 0)
    (`self.BackTrace` (`local.CurrentLoc`) (`local.ToCheck`) (`local.BridgeTiles`) (`local.PathTiles`))
    (goto _label)
    (else
      (return (`local.PathTiles`) (`local.EndPaths`)))))

(fn `GetNeighbourCount`
  (params (CurrentLocation :type "IntPoint Structure (by ref)") (PathTiles :type "Set of IntPoint Structure (by ref)"))
  (returns (Count :type Integer))
  (locals (Counter :type Integer))
  (for _array_element (`self.GetNeighbourLocation` CurrentLocation 1)
    (if (`BlueprintSetLibrary.Set_Contains` (`local.PathTiles`) _array_element)
      (set `local.Counter` (+ (`local.Counter`) 1))))
  (return (`local.Counter`)))

(fn `SpawnMazeMeshes`
  (locals (LoopLocation :type "IntPoint Structure") (`Loop Index` :type Integer) (SegmentIndex :type "Array of Boolean"))
  (bind (_size_x _size_y) (break `IntPoint` (`self.Size`)))
  (for _index (range (+ _size_x 1))
    (for _index_2 (range (+ _size_y 1))
      (set `local.LoopLocation` (make `IntPoint` _index _index_2))
      (if (`BlueprintSetLibrary.Set_Contains` (`self.Path Tiles`) (`local.LoopLocation`))
        ;[1 1 1] FloorTiles Generation - If has end path then spawn green tile other wise normal tile
        (message `/Game/MazeTask/MT_Blueprints/BPI_IntanceManager.AddNewMeshInstance` (`self.InsatanceManager`) (select `bool` (`BlueprintSetLibrary.Set_Contains` (`self.End Paths`) (`local.LoopLocation`)) :`false` "/Game/MazeTask/MT_Meshes/MT_Simple_GroundTile.MT_Simple_GroundTile" :`true` "/Game/MazeTask/MT_Meshes/MT_Simple_GroundTile.MT_Simple_GroundTile" :!type "StaticMesh Object Reference") (`self.BuildTileLocation` (`local.LoopLocation`)))
        (else
          ;[1 1 1] Way
          (message `/Game/MazeTask/MT_Blueprints/BPI_IntanceManager.AddNewMeshInstance` (`self.InsatanceManager`) "/Game/MazeTask/MT_Meshes/MT_WallTop.MT_WallTop" (`self.BuildTileLocation` (`local.LoopLocation`)))
          ;[1 1 1] Walls
          (message `/Game/MazeTask/MT_Blueprints/BPI_IntanceManager.AddNewMeshInstance` (`self.InsatanceManager`) "/Game/MazeTask/MT_Meshes/Walls.Walls" (`self.BuildTileLocation` (`local.LoopLocation`) 800.0 1)))))))

(fn `UserConstructionScript`)