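; BP_Chair is a chair actor that can be clicked to delete and has partly wired mouse-drag rotation.
; Clicking the Chair component traces under the cursor on the Visibility channel and destroys the hit actor.
; MouseMove yaws the chair by the inverted horizontal mouse delta while CanRotate is true, and EndRotate clears that flag.
; StartRotate is empty, with its flag and start-location setup left disconnected, so this graph never enables rotation.
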(event `Start Rotate`
  (params (MouseLocation :type "Vector2D Structure")))

(event `End Rotate`
  (set `self.CanRotate` false))

(event `Mouse Move`
  (params (MouseLocation :type "Vector2D Structure"))
  (if (`self.CanRotate`)
    (`SceneComponent.K2_AddWorldRotation` (`self.Chair`) (`KismetMathLibrary.MakeRotator` 0.0 0.0 (* (`KismetMathLibrary.BreakVector2D` (- MouseLocation (`self.StartRotateLocation`))) -1.0)) false false)
    (set `self.StartRotateLocation` MouseLocation)))

(event `self.Chair.OnClicked`
  (params (TouchedComponent :type "PrimitiveComponent Object Reference") (ButtonPressed :type "Key Structure"))
  (`self.K2_DestroyActor` (`.HitActor` (`GameplayStatics.BreakHitResult` (`PlayerController.GetHitResultUnderCursorByChannel` (`GameplayStatics.GetPlayerController` 0) "TraceTypeQuery1" true)))))

(fn `UserConstructionScript`)